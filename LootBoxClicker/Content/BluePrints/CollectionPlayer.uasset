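; CollectionPlayer is a player Blueprint that shows the collection UI and switches between the Collection and Tap levels.
; On BeginPlay it adds a CollectionWidget to the viewport, creates an unused TapScreenWidget, and stores the TapScreen component's widget, cast to CollectionWidget, in TapScreenRef.
; Input actions open levels by name, with TapScreenKey loading Collection and CollectionScreenKey loading Tap, the reverse of their names.
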(event `self.ReceiveBeginPlay`
  (bind _returnvalue (`|CreateWidget` "/Game/BluePrints/CollectionWidget.CollectionWidget_C" (`GameplayStatics.GetPlayerController` 0)))
  (`UserWidget.AddToViewport` _returnvalue 0)
  (`|CreateWidget` "/Game/BluePrints/TapScreenWidget.TapScreenWidget_C")
  (bind _ascollection_widget (cast `/Game/BluePrints/CollectionWidget` (`WidgetComponent.GetUserWidgetObject` (`self.TapScreen`))))
  (set `self.TapScreenRef` _ascollection_widget))

(event `InputAction|TapScreenKey`
  (params (Key :type "Key Structure"))
  (:`Pressed`
    (`GameplayStatics.OpenLevel` "Collection")))

(event `InputAction|CollectionScreenKey`
  (params (Key :type "Key Structure"))
  (:`Pressed`
    (`GameplayStatics.OpenLevel` "Tap")))

(fn `UserConstructionScript`)