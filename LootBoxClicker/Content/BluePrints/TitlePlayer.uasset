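; TitlePlayer is the player Blueprint for the title screen, setting up the main menu and its input.
; On BeginPlay it shows the mouse cursor, enables a virtual cursor, adds the widget from its MainMenu component to the viewport and plays the menu music.
; Escape quits the game, and the gamepad Special Right button opens the LootboxScreen level.
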(event `self.ReceiveBeginPlay`
  (bind _returnvalue (`GameplayStatics.GetPlayerController` 0))
  (set `PlayerController.bShowMouseCursor` true _returnvalue)
  (`VirtualCursorFunctionLibrary.EnableVirtualCursor` _returnvalue)
  (`UserWidget.AddToViewport` (`WidgetComponent.GetWidget` (`self.MainMenu`)) 0)
  (`GameplayStatics.PlaySound2D` "/Game/SoundEffects/MenuBGM.MenuBGM" 1.0 1.0 0.0 null null))

(event `Key|Escape`
  (params (Key :type "Key Structure"))
  (:`Pressed`
    (`KismetSystemLibrary.QuitGame` null "Quit")))

(event `Key|Gamepad_Special_Right`
  (params (Key :type "Key Structure"))
  (:`Pressed`
    (`GameplayStatics.OpenLevel` "LootboxScreen")))

(fn `UserConstructionScript`)