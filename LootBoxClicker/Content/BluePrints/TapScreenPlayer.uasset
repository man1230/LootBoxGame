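; Player Blueprint that runs a widget-driven tap game, switching between tap, lootbox and collection screens.
; BeginPlay starts music, enables a virtual cursor and creates all widgets up front, passing the collection to the lootbox and the lootbox to the tap screen.
; T or right shoulder cycles screens by toggling visibility through an integer state.
; G or gamepad special-right toggles the pause menu, freezing global time dilation, and Escape quits.
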(event `self.ReceiveBeginPlay`
  (`GameplayStatics.PlaySound2D` "/Game/SoundEffects/BGM.BGM" 1.0 1.0 0.0 null null)
  (`VirtualCursorFunctionLibrary.EnableVirtualCursor` (`GameplayStatics.GetPlayerController` 0))
  (bind _returnvalue (`|CreateWidget` "/Game/BluePrints/PauseMenu.PauseMenu_C"))
  (bind _returnvalue_2 (`|CreateWidget` "/Game/BluePrints/CollectionWidget.CollectionWidget_C"))
  (bind _output_get (set `self.CollectionWid` _returnvalue_2))
  (bind _returnvalue_3 (`|CreateWidget` "/Game/BluePrints/Lootbox.Lootbox_C" null _output_get))
  (bind _returnvalue_4 (`|CreateWidget` "/Game/BluePrints/TapScreenWidget.TapScreenWidget_C" null _returnvalue_3))
  (`UserWidget.AddToViewport` _returnvalue_3 0)
  (`UserWidget.AddToViewport` _returnvalue_2 0)
  (`UserWidget.AddToViewport` _returnvalue_4 0)
  (`Widget.SetVisibility` _returnvalue_4 "Collapsed")
  (`Widget.SetVisibility` _returnvalue_2 "Collapsed")
  (`UserWidget.AddToViewport` _returnvalue 0)
  (`Widget.SetVisibility` _returnvalue "Collapsed"))

(event `Key|T`
  (params (Key :type "Key Structure"))
  (bind _switch (`self.switch`))
  (:`Pressed`
    (`/Engine/EditorBlueprintResources/StandardMacros.CompareInt` _switch :!label _label
      (:`>`
        (`/Engine/EditorBlueprintResources/StandardMacros.CompareInt` _switch 1
          (:`>`
            (`/Engine/EditorBlueprintResources/StandardMacros.CompareInt` _switch 2
              (:`==`
                _)
              (:`<`
                _))
            (bind _output_get (set `self.switch` 0 :!label _label_2))
            (`Widget.SetVisibility` (stale `self.ReceiveBeginPlay` _returnvalue_2) "Hidden")
            (`Widget.SetVisibility` (stale `self.ReceiveBeginPlay` _returnvalue_3) "Hidden")
            (`Widget.SetVisibility` (stale `self.ReceiveBeginPlay` _returnvalue_4) "Visible"))
          (:`==`
            (bind _output_get_2 (set `self.switch` 2))
            (`Widget.SetVisibility` (stale `self.ReceiveBeginPlay` _returnvalue_3) "Hidden")
            (`Widget.SetVisibility` (stale `self.ReceiveBeginPlay` _returnvalue_4) "Hidden")
            (`Widget.SetVisibility` (stale `self.ReceiveBeginPlay` _returnvalue_2) "Visible"))))
      (:`==`
        (bind _output_get_3 (set `self.switch` 1))
        (`Widget.SetVisibility` (stale `self.ReceiveBeginPlay` _returnvalue_4) "Collapsed")
        (`Widget.SetVisibility` (stale `self.ReceiveBeginPlay` _returnvalue_2) "Collapsed")
        (`Widget.SetVisibility` (stale `self.ReceiveBeginPlay` _returnvalue_3) "Visible"))
      (:`<`
        (goto _label_2)))))

(event `Key|Q`
  (params (Key :type "Key Structure")))

(event `Key|Gamepad_RightShoulder`
  (params (Key :type "Key Structure"))
  (:`Pressed`
    (goto _label)))

(event `Key|Escape`
  (params (Key :type "Key Structure"))
  (:`Pressed`
    (`KismetSystemLibrary.QuitGame` null "Quit")))

(event `Key|Y`
  (params (Key :type "Key Structure")))

(event `Key|U`
  (params (Key :type "Key Structure")))

(event `Key|G`
  (params (Key :type "Key Structure"))
  (:`Pressed`
    (if (`self.notvisible`) :!label _label_3
      (`Widget.SetVisibility` (stale `self.ReceiveBeginPlay` _returnvalue) "Visible")
      (set `self.notvisible` false)
      (`GameplayStatics.SetGlobalTimeDilation` 0.0)
      (else
        (`Widget.SetVisibility` (stale `self.ReceiveBeginPlay` _returnvalue) "Collapsed")
        (set `self.notvisible` true)
        (`GameplayStatics.SetGlobalTimeDilation` 1.0)))))

(event `Key|Gamepad_Special_Right`
  (params (Key :type "Key Structure"))
  (:`Pressed`
    (goto _label_3)))

(fn `UserConstructionScript`)