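; Player Blueprint for a tap-screen game that creates and switches between the tap screen, lootbox and collection widgets.
; BeginPlay shows the mouse cursor and chains widget references from collection to lootbox to tap screen, leaving only the lootbox visible.
; T cycles lootbox, collection and tap screen through nested integer compares on Switch, printing each new value.
; Escape quits the game.
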(event `self.ReceiveBeginPlay`
  (set `PlayerController.bShowMouseCursor` true (`GameplayStatics.GetPlayerController` 0))
  (bind _returnvalue (`|CreateWidget` "/Game/BluePrints/CollectionWidget.CollectionWidget_C"))
  (bind _output_get (set `self.CollectionWid` _returnvalue))
  (bind _returnvalue_2 (`|CreateWidget` "/Game/BluePrints/Lootbox.Lootbox_C" null _output_get))
  (bind _returnvalue_3 (`|CreateWidget` "/Game/BluePrints/TapScreenWidget.TapScreenWidget_C" null _returnvalue_2))
  (`UserWidget.AddToViewport` _returnvalue_2 0)
  (`UserWidget.AddToViewport` _returnvalue 0)
  (`UserWidget.AddToViewport` _returnvalue_3 0)
  (`Widget.SetVisibility` _returnvalue_3 "Collapsed")
  (`Widget.SetVisibility` _returnvalue "Collapsed"))

(event `Key|T`
  (params (Key :type "Key Structure"))
  (bind _switch (`self.switch`))
  (:`Pressed`
    (`/Engine/EditorBlueprintResources/StandardMacros.CompareInt` _switch
      (:`>`
        (`/Engine/EditorBlueprintResources/StandardMacros.CompareInt` _switch 1
          (:`>`
            (`/Engine/EditorBlueprintResources/StandardMacros.CompareInt` _switch 2
              (:`==`
                _)
              (:`<`
                _))
            (bind _output_get (set `self.switch` 0 :!label _label))
            (`KismetSystemLibrary.PrintString` (`KismetStringLibrary.Conv_IntToString` _output_get))
            (`Widget.SetVisibility` (stale `self.ReceiveBeginPlay` _returnvalue) "Hidden")
            (`Widget.SetVisibility` (stale `self.ReceiveBeginPlay` _returnvalue_2) "Hidden")
            (`Widget.SetVisibility` (stale `self.ReceiveBeginPlay` _returnvalue_3) "Visible"))
          (:`==`
            (bind _output_get_2 (set `self.switch` 2))
            (`KismetSystemLibrary.PrintString` (`KismetStringLibrary.Conv_IntToString` _output_get_2))
            (`Widget.SetVisibility` (stale `self.ReceiveBeginPlay` _returnvalue_2) "Hidden")
            (`Widget.SetVisibility` (stale `self.ReceiveBeginPlay` _returnvalue_3) "Hidden")
            (`Widget.SetVisibility` (stale `self.ReceiveBeginPlay` _returnvalue) "Visible"))))
      (:`==`
        (bind _output_get_3 (set `self.switch` 1))
        (`KismetSystemLibrary.PrintString` (`KismetStringLibrary.Conv_IntToString` _output_get_3))
        (`Widget.SetVisibility` (stale `self.ReceiveBeginPlay` _returnvalue_3) "Collapsed")
        (`Widget.SetVisibility` (stale `self.ReceiveBeginPlay` _returnvalue) "Collapsed")
        (`Widget.SetVisibility` (stale `self.ReceiveBeginPlay` _returnvalue_2) "Visible"))
      (:`<`
        (goto _label)))))

(event `Key|Q`
  (params (Key :type "Key Structure")))

(event `Key|Escape`
  (params (Key :type "Key Structure"))
  (:`Pressed`
    (`KismetSystemLibrary.QuitGame` null "Quit")))

(event `Key|Y`
  (params (Key :type "Key Structure")))

(event `Key|U`
  (params (Key :type "Key Structure")))

(fn `UserConstructionScript`)